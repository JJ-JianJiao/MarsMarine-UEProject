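; Alien enemy that chases the player's marine and plays a melee attack montage when in range.
; A looping AIMoveTo drives pursuit, while Tick triggers attacks, pausing movement until the montage completes, and halts the alien once the marine dies.
; Damage lowers clamped health; at zero the alien disables movement and collision, credits the marine's kill and registers with BP_GameMode.
; DamagePlayer is not called within this Blueprint, and the delayed destroy is unwired.
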(event `self.ReceiveBeginPlay`
  (bind _asbp_marine (cast `/Game/Blueprints/Pawns/BP_Marine` (`GameplayStatics.GetPlayerCharacter` 0)))
  (bind _output_get (set `self.BP_Marine` _asbp_marine))
  (if (and (not (`/Game/Blueprints/Pawns/BP_Marine.Dead` (`self.BP_Marine`))) (not (`self.Dead`))) :!label _label
    (`|AIMoveTo` self (0.0 0.0 0.0) _output_get
      (:`OnSuccess`
        _)
      (:`OnFail`
        _))
    (`KismetSystemLibrary.Delay` 0.2)
    (goto _label)))

(event `self.ReceiveTick`
  (params (DeltaSeconds :type "Float (single-precision)"))
  (if (`/Game/Blueprints/Pawns/BP_Marine.Dead` (`self.BP_Marine`))
    (`MovementComponent.StopMovementImmediately` (`self.CharacterMovement`))
    (elif (`self.Can attack`)
      (`self.Deactivate AI Movement`)
      (`|PlayMontage` (`self.Mesh`) "/Game/Characters/Enemy_Great_Spider/Animations/AlienAttack1.AlienAttack1"
        (:`OnCompleted`
          (`self.Activate AI Movement`))))))

(event `self.ReceiveAnyDamage`
  (params (Damage :type "Float (single-precision)") (DamageType :type "DamageType Object Reference") (InstigatedBy :type "Controller Object Reference") (DamageCauser :type "Actor Object Reference"))
  (bind _returnvalue (`self.Decrease Health` Damage))
  (bind _returnvalue_2 (<= _returnvalue 0.0))
  (if _returnvalue_2
    (set `self.Dead` _returnvalue_2)
    (`self.Kill AI`)))

(fn `Activate AI Movement`
  (`ActorComponent.Activate` (`self.CharacterMovement`) false))

(fn `Can attack`
  (returns (ReturnValue :type Boolean))
  (return (and (`self.Is Within Attack Range`) (not (`self.Is Attacking`)) (not (`self.Dead`)))))

(fn `Damage Player`
  (`GameplayStatics.ApplyDamage` (`GameplayStatics.GetPlayerCharacter` 0) (`self.Damage Per hit`)))

(fn `Deactivate AI Movement`
  (bind _charactermovement (`self.CharacterMovement`))
  (`MovementComponent.StopMovementImmediately` _charactermovement)
  (`ActorComponent.Deactivate` _charactermovement))

(fn `Decrease Health`
  (params (Damage :type "Float (double-precision)"))
  (returns (ReturnValue :type "Float (double-precision)"))
  (`KismetSystemLibrary.PrintString` "Get Damage")
  (bind _output_get (set `self.Health` (`KismetMathLibrary.FClamp` (- (`self.Health`) Damage) 0.0 100.0)))
  (return _output_get))

(fn `Is Attacking`
  (returns (ReturnValue :type Boolean))
  (return (`AnimInstance.Montage_IsPlaying` (`SkeletalMeshComponent.GetAnimInstance` (`self.Mesh`)) "/Game/Characters/Enemy_Great_Spider/Animations/AlienAttack1.AlienAttack1")))

(fn `Is Within Attack Range`
  (returns (ReturnValue :type Boolean))
  (return (<= (`self.GetDistanceTo` (`GameplayStatics.GetPlayerCharacter` 0)) (`self.AttackRange`))))

(fn `Kill AI`
  (set `self.Dead` true)
  (`self.Deactivate AI Movement`)
  (`self.SetActorEnableCollision` false)
  (`/Game/Blueprints/Pawns/BP_Marine.Increase Kills` (`self.BP_Marine`))
  (bind _asbp_game_mode (cast `/Game/Blueprints/GameMode/BP_GameMode` (`GameplayStatics.GetGameMode`)))
  (`/Game/Blueprints/GameMode/BP_GameMode.Register Alien Death` _asbp_game_mode self))

(fn `UserConstructionScript`)